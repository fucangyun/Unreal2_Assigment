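; Goblin NPC Blueprint that relays what it senses to its AI controller, BP_AICon.
; Its pawn sensing component passes seen pawns on as the target actor, and passes noise locations on as the target location when the volume exceeds a fixed threshold.
; SetDestination lets a caller push a target location to the same controller directly.
; The Blueprint holds no movement or decision logic of its own.
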(event OnSeePawn(MyPawnSensing)
  (params (Pawn :type Pawn%20Object%20Reference))
  (bind _asbp_aicon (Utilities|Casting|CastToBP_AICon (AI|GetAIController self)))
  (Default|UpdateTargetActor _asbp_aicon Pawn))

(event OnHearNoise(MyPawnSensing)
  (params (Instigator :type Pawn%20Object%20Reference) (Location :type Vector%20%28by%20ref%29 :default "0, 0, 0") (Volume :type Float%20%28single-precision%29))
  (if (> Volume 3e+02)
    (bind _asbp_aicon (Utilities|Casting|CastToBP_AICon (AI|GetAIController self)))
    (Default|UpdateTargetLocation _asbp_aicon Location)))

(event EventBeginPlay
  (|CallParentFunction) ; This node is disabled and will not be called.\nDrag off pins to build functionality.
)

(event Collision|EventActorBeginOverlap
  (params (OtherActor :type Actor%20Object%20Reference))
  (|CallParentFunction OtherActor) ; This node is disabled and will not be called.\nDrag off pins to build functionality.
)

(event EventTick
  (params (DeltaSeconds :type Float%20%28single-precision%29))
  (|CallParentFunction DeltaSeconds) ; This node is disabled and will not be called.\nDrag off pins to build functionality.
)

(fn ConstructionScript
  (|CallParentFunction))

(fn SetDestination
  (params (Destination :type Vector :default "0, 0, 0"))
  (bind _asbp_aicon (Utilities|Casting|CastToBP_AICon (AI|GetAIController self)))
  (Default|UpdateTargetLocation _asbp_aicon Destination))