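; Wave spawner that creates batches of BP_EnemyCharacter enemies over a set number of rounds.
; GoblinFactory line-traces vertically through the spawner and spawns each enemy at a random navigable point within Radius, with debug drawing enabled.
; A Delay-throttled Tick prunes dead enemies from the tracked array and flags IsAllDead once it empties, which is never reset here.
; That flag triggers further rounds, then a one-time RoundsFInish call when none remain.
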(event EventBeginPlay
  (if (> (Variables|Default|GetRounds) 1)
    (CallFunction|GoblinFactory)))

(event Collision|EventActorBeginOverlap
  (params (OtherActor :type Actor%20Object%20Reference)))

(event EventTick
  (params (DeltaSeconds :type Float%20%28single-precision%29))
  (bind _spawnedenemies (Variables|Default|GetSpawnedEnemies))
  (Utilities|FlowControl|Delay 1.0)
  (if (Variables|Default|GetIsAllDead)
    (if (> (Variables|Default|GetRounds) 0)
      (bind _result (Math|Integer|DecrementInt (Variables|Default|GetRounds))
        (:%20%20
          (Variables|Default|SetRounds _result)
          (CallFunction|GoblinFactory)))
      (else
        (Utilities|FlowControl|DoOnce false
          (:Completed
            (Default|CallCallRoundsFInish)))))
    (elif (> (Utilities|Array|Length _spawnedenemies) 0)
      (for _array_element _spawnedenemies
        (if (not (Default|IsAlive _array_element))
          (Utilities|Array|RemoveItem _spawnedenemies _array_element)))
      (else
        (Variables|Default|SetIsAllDead true)))))

(fn ConstructionScript)

(fn GoblinFactory
  (bind _returnvalue (Transformation|GetActorLocation))
  (bind _returnvalue_2 (Transformation|GetActorTransform))
  (bind _num (Variables|Default|GetNum))
  (if (> _num 0)
    (Utilities|Array|Clear (Variables|Default|GetSpawnedEnemies))
    (for _index (range 0 (- _num 1))
      (bind (_outhit _returnvalue_3) (Collision|LineTraceForObjects (+ _returnvalue "0.000000,0.000000,1000.000000") (- _returnvalue "0.000000,0.000000,1000.000000") (Utilities|Array|MakeArray "ObjectTypeQuery2" "ObjectTypeQuery1") false 0 "Persistent"))
      (if _returnvalue_3
        (bind _randomlocation (Class|NavigationSystemV1|GetRandomLocationinNavigableRadius (.Location (Collision|BreakHitResult _outhit)) (Variables|Default|GetRadius) 0 0))
        (Rendering|Debug|DrawDebugSphere _randomlocation 1e+02 2 "(R=0.000000,G=1.000000,B=0.090994,A=1.000000)" 5.0 2.0)
        (bind _returnvalue_4 (Game|SpawnActorfromClass (Variables|Default|GetEnemyClass) (Math|Transform|MakeTransform _randomlocation (.rotation _returnvalue_2) (.scale _returnvalue_2)) "Undefined" self 0))
        (bind _asbp_enemy_character (Utilities|Casting|CastToBP_EnemyCharacter _returnvalue_4))
        (Utilities|Array|Add (Variables|Default|GetSpawnedEnemies) _asbp_enemy_character)))))