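; Anim notify state that marks the active attack window of a character's weapon within an animation.
; On begin, it casts the mesh owner to BP_Character and calls BeginWeaponAttack on a valid CurrentWeapon, passing the notify's Damage value.
; On end, it calls EndWeaponAttack on the owner's current weapon to close the window.
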(fn ReceivedNotifyBegin
  (params (MeshComp :type Skeletal%20Mesh%20Component%20Object%20Reference) (Animation :type Anim%20Sequence%20Base%20Object%20Reference) (TotalDuration :type Float%20%28single-precision%29) (EventReference :type Anim%20Notify%20Event%20Reference%20Structure%20%28by%20ref%29))
  (bind _asbp_character (Utilities|Casting|CastToBP_Character (Components|GetOwner MeshComp)))
  (Utilities|IsValid (Variables|/Game/Assets/Blueprints/Character/BP_PlayerCharacter.BP_PlayerCharacter_C|GetCurrentWeapon _asbp_character)
    (:Is%20Valid
      (Default|BeginWeaponAttack (Variables|/Game/Assets/Blueprints/Character/BP_PlayerCharacter.BP_PlayerCharacter_C|GetCurrentWeapon _asbp_character) (Variables|Config|GetDamage))
      (return true))))

(fn ReceivedNotifyEnd
  (params (MeshComp :type Skeletal%20Mesh%20Component%20Object%20Reference) (Animation :type Anim%20Sequence%20Base%20Object%20Reference) (EventReference :type Anim%20Notify%20Event%20Reference%20Structure%20%28by%20ref%29))
  (bind _asbp_character (Utilities|Casting|CastToBP_Character (Components|GetOwner MeshComp)))
  (Utilities|IsValid (Variables|/Game/Assets/Blueprints/Character/BP_PlayerCharacter.BP_PlayerCharacter_C|GetCurrentWeapon _asbp_character)
    (:Is%20Valid
      (Default|EndWeaponAttack (Variables|/Game/Assets/Blueprints/Character/BP_PlayerCharacter.BP_PlayerCharacter_C|GetCurrentWeapon _asbp_character))
      (return false))))